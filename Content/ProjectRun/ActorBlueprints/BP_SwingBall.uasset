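; BP_SwingBall is a swinging-ball obstacle that knocks run characters away on contact.
; A timeline started at BeginPlay drives the static mesh's relative roll to produce the swing.
; On a mesh hit, the server fires the RadialForce impulse and launches the RunCharacter using force strength on all three axes, independent of hit direction.
; An AddImpulse function repeats this launch for player 0 but is only called from unconnected nodes.
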(event OnComponentBeginOverlap(StaticMesh)
  (params (OverlappedComponent :type Primitive%20Component%20Object%20Reference) (OtherActor :type Actor%20Object%20Reference) (OtherComp :type Primitive%20Component%20Object%20Reference) (OtherBodyIndex :type Integer) (bFromSweep :type Boolean) (SweepResult :type Hit%20Result%20Structure%20%28by%20ref%29)))

(event OnComponentHit(StaticMesh)
  (params (HitComponent :type Primitive%20Component%20Object%20Reference) (OtherActor :type Actor%20Object%20Reference) (OtherComp :type Primitive%20Component%20Object%20Reference) (NormalImpulse :type Vector :default "0, 0, 0") (Hit :type Hit%20Result%20Structure%20%28by%20ref%29))
  (bind _radialforce (Variables|Default|GetRadialForce))
  (Networking|SwitchHasAuthority
    (:Authority
      (bind _asrun_character (Utilities|Casting|CastToRunCharacter OtherActor))
      (Class|RadialForceComponent|FireImpulse _radialforce)
      (Character|LaunchCharacter _asrun_character (Math|Conversions|ToVector(Float) (Variables|/Script/Engine.RadialForceComponent|GetForceStrength _radialforce)) false false))))

(event EventBeginPlay
  (bind _새_트랙_2 (Timeline|타임라인_0 Play)
    (:Update
      (Transformation|SetRelativeRotation (Variables|Default|GetStaticMesh) (Math|Rotator|MakeRotator _새_트랙_2 0.0 0.0) false false))))

(fn ConstructionScript)

(fn AddImpulse
  (params (A :type Object%20Object%20Reference))
  (bind _returnvalue (Game|GetPlayerCharacter 0))
  (bind _radialforce (Variables|Default|GetRadialForce))
  (if (== A _returnvalue)
    (Class|RadialForceComponent|FireImpulse _radialforce)
    (Character|LaunchCharacter _returnvalue (Math|Conversions|ToVector(Float) (Variables|/Script/Engine.RadialForceComponent|GetForceStrength _radialforce)) false false)))