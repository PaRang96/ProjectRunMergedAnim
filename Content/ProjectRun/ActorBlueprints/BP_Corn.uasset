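; BP_Corn is an obstacle whose spinner mesh moves along Z and launches RunCharacters upward on hit, server-side only.
; After a random BeginPlay delay, a PlayRate timeline scales SpinnerLocation's rate by SpinnerSpeed and restarts it every update.
; SpinnerLocation's track, named Rotation, drives the mesh's relative Z location.
; The delay is rolled without an authority check, and its OnRep is empty.
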(event OnComponentHit(SM_Spinner_V1)
  (params (HitComponent :type Primitive%20Component%20Object%20Reference) (OtherActor :type Actor%20Object%20Reference) (OtherComp :type Primitive%20Component%20Object%20Reference) (NormalImpulse :type Vector :default "0, 0, 0") (Hit :type Hit%20Result%20Structure%20%28by%20ref%29))
  (Networking|SwitchHasAuthority
    (:Authority
      (bind _asrun_character (Utilities|Casting|CastToRunCharacter OtherActor))
      (Character|LaunchCharacter _asrun_character "0.000000,0.000000,500.000000" false false))))

(event EventBeginPlay
  (bind _output_get (Variables|Default|SetDelay (Math|Random|RandomFloatinRange 1.0 3.0)))
  (Utilities|FlowControl|Delay _output_get)
  (bind _speed (Timeline|PlayRate Play)
    (:Update
      (Components|Timeline|SetPlayRate (Variables|Default|GetSpinnerLocation) (* _speed (Variables|Default|GetSpinnerSpeed)))
      (bind _rotation (Timeline|SpinnerLocation PlayFromStart)
        (:Update
          (Transformation|SetRelativeLocation (Variables|Default|GetSM_Spinner_V1) (Math|Vector|MakeVector 0.0 0.0 _rotation) false false))))))

(fn ConstructionScript)

(fn OnRepDelay)