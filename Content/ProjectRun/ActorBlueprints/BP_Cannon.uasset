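; BP_Cannon is a cannon actor that fires BP_Bullet actors from three arrow components at random intervals.
; BeginPlay starts three timelines in parallel collapsed graphs, one per arrow.
; Each timeline's Update feeds a random 1–3 second Delay before spawning a bullet at its arrow's transform, so the pending Delay throttles the per-frame updates.
; All three lanes write one shared Delay variable, whose OnRep is empty.
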(event EventBeginPlay
  (Utilities|FlowControl|Sequence
    (:then_0
      (|CollapseGraph_0))
    (:then_1
      (|CollapseGraph_1))
    (:then_2
      (|CollapseGraph_2))))

(event EventTick
  (params (DeltaSeconds :type Float%20%28single-precision%29)))

(event Input|MouseEvents|LeftMouseButton
  (params (Key :type Key%20Structure :default "None")))

(fn ConstructionScript)

(fn OnRepDelay)