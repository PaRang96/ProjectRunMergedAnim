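; BP_Goal is the finish-line trigger that records which players reach the goal.
; When its Cube component is overlapped, the server checks that the overlapping component is the capsule of an InheritRunCharacter.
; It then adds that character's BP_RunPlayerController to the PlayerRanking array in BP_RunGameMode with AddUnique, so arrival order forms the ranking without duplicates.
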(event OnComponentBeginOverlap(Cube)
  (params (OverlappedComponent :type Primitive%20Component%20Object%20Reference) (OtherActor :type Actor%20Object%20Reference) (OtherComp :type Primitive%20Component%20Object%20Reference) (OtherBodyIndex :type Integer) (bFromSweep :type Boolean) (SweepResult :type Hit%20Result%20Structure%20%28by%20ref%29))
  (Networking|SwitchHasAuthority
    (:Authority
      (bind _asinherit_run_character (Utilities|Casting|CastToInheritRunCharacter OtherActor))
      (if (== (Variables|/Script/Engine.Character|GetCapsuleComponent _asinherit_run_character) OtherComp)
        (bind _asbp_run_player_controller (Utilities|Casting|CastToBP_RunPlayerController (Pawn|GetController _asinherit_run_character)))
        (bind _asbp_run_game_mode (Utilities|Casting|CastToBP_RunGameMode (Game|GetGameMode)))
        (Utilities|Array|AddUnique (Variables|/Game/ProjectRun/GameMode/RunGame/BP_RunGameMode.BP_RunGameMode_C|GetPlayerRanking _asbp_run_game_mode) _asbp_run_player_controller)))))

(fn ConstructionScript)