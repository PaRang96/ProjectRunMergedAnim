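; Game mode for the run race that steps the RunGameState enum through four phases, polled every Tick.
; The first phase waits until player count equals the game instance's Slots, and the next until BP_Goal's ranking has an entry.
; It then enters Finish, calls FinishCount on the first player's HUD only, and advances after a delay.
; Input-disabling logic exists but is unconnected.
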(event EventBeginPlay
  (Variables|/Game/ProjectRun/GameMode/RunGameState.RunGameState_C|SetEN_GameSate (CallFunction|GetRunGameState) "NewEnumerator0"))

(event EventTick
  (params (DeltaSeconds :type Float%20%28single-precision%29))
  (bind _asrun_game_state (CallFunction|GetRunGameState))
  (bind _asrun_game_state_2 (CallFunction|GetRunGameState))
  (Utilities|FlowControl|Sequence
    (:then_0
      (if (Utilities|Enum|Equal(Enum) (Variables|/Game/ProjectRun/GameMode/RunGameState.RunGameState_C|GetEN_GameSate (CallFunction|GetRunGameState)) "NewEnumerator0")
        (bind _asrun_game_instance (Utilities|Casting|CastToRunGameInstance (Game|GetGameInstance)))
        (bind _returnvalue (Class|GameModeBase|GetNumPlayers))
        (if (== _returnvalue (Variables|/Game/ProjectRun/GameMode/RunGameInstance.RunGameInstance_C|GetSlots _asrun_game_instance))
          (Variables|/Game/ProjectRun/GameMode/RunGameState.RunGameState_C|SetEN_GameSate (CallFunction|GetRunGameState) "NewEnumerator1"))))
    (:then_1
      (if (Utilities|Enum|Equal(Enum) (Variables|/Game/ProjectRun/GameMode/RunGameState.RunGameState_C|GetEN_GameSate _asrun_game_state_2) "NewEnumerator1")
        (if (CallFunction|FirstPlayerPassed)
          (Utilities|FlowControl|Sequence
            (:then_0
              (Variables|/Game/ProjectRun/GameMode/RunGameState.RunGameState_C|SetEN_GameSate _asrun_game_state_2 "NewEnumerator2")
              (Development|PrintString "Game State: Finish" true true "(R=0.117151,G=0.173611,B=0.110445,A=1.000000)" 5e+01))
            (:then_1
              (bind _asbp_run_player_controller (CallFunction|GetAllPlayerControllers))
              (bind _asbp_run_hud (Utilities|Casting|CastToBP_RunHUD (HUD|GetHUD _asbp_run_player_controller)))
              (Default|FinishCount _asbp_run_hud))))))
    (:then_2
      (if (Utilities|Enum|Equal(Enum) (Variables|/Game/ProjectRun/GameMode/RunGameState.RunGameState_C|GetEN_GameSate _asrun_game_state) "NewEnumerator2")
        (Utilities|FlowControl|Delay 6e+01)
        (Variables|/Game/ProjectRun/GameMode/RunGameState.RunGameState_C|SetEN_GameSate _asrun_game_state "NewEnumerator3")))))

(fn ConstructionScript)

(fn FirstPlayerPassed
  (bind _returnvalue (Actor|GetActorOfClass "/Game/ProjectRun/ActorBlueprints/BP_Goal.BP_Goal_C"))
  (return (> (Utilities|Array|Length (Variables|/Game/ProjectRun/ActorBlueprints/BP_Goal.BP_Goal_C|GetPlayerRanking _returnvalue)) 0)))

(fn GetRunGameState
  (bind _asrun_game_state (Utilities|Casting|CastToRunGameState (Game|GetGameState)))
  (return _asrun_game_state))

(fn GetAllPlayerControllers
  (bind _returnvalue (Class|GameModeBase|GetNumPlayers))
  (for _index (range 0 (- _returnvalue 1))
    (bind _asbp_run_player_controller (Utilities|Casting|CastToBP_RunPlayerController (Game|GetPlayerController _index)))
    (return _asbp_run_player_controller))
  (return _asbp_run_player_controller))