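; BP_RunPlayerController is the run game mode's player controller, handling player number handoff and movement shutdown.
; On possess, ResClientPossess reads Slots from RunGameInstance and passes it through ReqSetPlayerNumber to the BP_RunPlayerState, a Res/Req naming that suggests a client-server round trip.
; SendDisableMovement deactivates the controlled InheritRunCharacter's movement component, then switches to UI-only input with a visible cursor.
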(event Custom|ResClientPossess
  (bind _asrun_game_instance (Utilities|Casting|CastToRunGameInstance (Game|GetGameInstance)))
  (CallFunction|ReqSetPlayerNumber (Variables|/Game/ProjectRun/GameMode/RunGameInstance.RunGameInstance_C|GetSlots _asrun_game_instance)))

(event Custom|ReqSetPlayerNumber
  (params (PlayerNumber :type Integer))
  (bind _asbp_run_player_state (Utilities|Casting|CastToBP_RunPlayerState (Variables|GetPlayerState)))
  (Default|GetPlayerNumber _asbp_run_player_state PlayerNumber))

(event Custom|SendDisableMovement
  (CallFunction|DisableMovement)
  (Input|SetInputModeUIOnly self 0 "DoNotLock")
  (Variables|Default|SetbShowMouseCursor true))

(event EventPossess
  (params (PossessedPawn :type Pawn%20Object%20Reference))
  (CallFunction|ResClientPossess))

(fn ConstructionScript)

(fn DisableMovement
  (bind _asinherit_run_character (Utilities|Casting|CastToInheritRunCharacter (Pawn|GetControlledPawn)))
  (Components|Activation|Deactivate (Variables|/Script/Engine.Character|GetCharacterMovement _asinherit_run_character)))