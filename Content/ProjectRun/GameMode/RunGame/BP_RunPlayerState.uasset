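; Player state for the Run game mode that holds a player's name, point score and player number, each with a RepNotify.
; Name and Point changes are relayed through event dispatchers, while PlayerNumber changes update the local BP_RunHUD directly.
; On BeginPlay it binds itself to that HUD, and a helper derives the player number by counting PlayerController actors.
; Debug prints show the score every tick and the player number when it replicates.
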(event EventBeginPlay
  (CallFunction|InitBind))

(event EventTick
  (params (DeltaSeconds :type Float%20%28single-precision%29))
  (Development|PrintString (Utilities|String|ToString(Integer) (Variables|Default|GetPoint)) true true "(R=0.000000,G=0.660000,B=1.000000,A=1.000000)" DeltaSeconds))

(fn ConstructionScript)

(fn OnRepName
  (Default|CallNameDispatcher (Variables|Default|GetName)))

(fn SetName
  (params (Name :type String))
  (Variables|Default|SetName Name))

(fn AddPoint
  (params (Point :type Integer))
  (Variables|Default|SetPoint (+ Point (Variables|Default|GetPoint))))

(fn OnRepPoint
  (Default|CallPointDispatcher (Variables|Default|GetPoint)))

(fn GetPlayerNumber
  (params (PlayerNumber :type Integer))
  (bind _outactors (Actor|GetAllActorsOfClass "/Script/Engine.PlayerController"))
  (Variables|Default|SetPlayerNumber (Utilities|Array|Length _outactors)))

(fn OnRepPlayerNumber
  (bind _playernumber (Variables|Default|GetPlayerNumber))
  (Development|PrintString (Utilities|String|ToString(Integer) _playernumber) true true "(R=1.000000,G=0.000000,B=0.059269,A=1.000000)" 6e+01)
  (bind _asbp_run_hud (Utilities|Casting|CastToBP_RunHUD (HUD|GetHUD (Game|GetPlayerController 0))))
  (Default|UpdatePlayerNumber _asbp_run_hud _playernumber))

(fn InitBind
  (bind _asbp_run_hud (Utilities|Casting|CastToBP_RunHUD (HUD|GetHUD (Game|GetPlayerController 0))))
  (Default|BindPlayerNumber _asbp_run_hud self))