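; Lobby player state that holds a player's replicated name and exposes it to the lobby UI.
; On BeginPlay it registers itself with the first player controller's BP_LobbyHUD through BindUserState.
; SetName writes the Name variable, and its RepNotify fires the ChangeName event dispatcher so bound listeners receive the new name.
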(event EventBeginPlay
  (CallFunction|InitBind))

(fn ConstructionScript)

(fn InitBind
  (bind _asbp_lobby_hud (Utilities|Casting|CastToBP_LobbyHUD (HUD|GetHUD (Game|GetPlayerController 0))))
  (Default|BindUserState _asbp_lobby_hud self))

(fn OnRepName
  (Default|CallEDChangeName (Variables|Default|GetName)))

(fn SetName
  (params (Name :type String))
  (Variables|Default|SetName Name))